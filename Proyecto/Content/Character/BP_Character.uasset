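; BP_Character is a Paper2D side-scrolling player character that runs along X and jumps.
; BeginPlay adds the Enhanced Input mapping context, and movement and jump actions drive movement and swap idle, run, rise and fall flipbooks, with landing restoring idle.
; Tick mirrors the sprite by X velocity, keeping the last facing when still.
; A constant branch on grounded movement release forces one facing, and a Y-axis position lock is left unconnected.
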(event Input|EnhancedActionEvents|EnhancedInputActionIA_Salto
  (params (ActionValue :type Boolean) (ElapsedSeconds :type Float%20%28double-precision%29) (TriggeredSeconds :type Float%20%28double-precision%29) (InputAction :type Input%20Action%20Object%20Reference :default "/Game/Character/Input/Action/IA_Salto.IA_Salto"))
  ;[1 1 1] SALTO
  (:Triggered
    (Character|Jump :!label _label)
    (Sprite|SetFlipbook (Variables|Default|GetSprite) "/Game/Assets/CHILLBOY_BASIC_ANIMATION/JUMP/SPR_CHILL_BOY_Jump_Up.SPR_CHILL_BOY_Jump_Up"))
  (:Ongoing
    (goto _label))
  (:Completed
    (Character|StopJumping)
    (Sprite|SetFlipbook (Variables|Default|GetSprite) "/Game/Assets/CHILLBOY_BASIC_ANIMATION/JUMP/SPR_CHILL_BOY_Jump_Fall.SPR_CHILL_BOY_Jump_Fall")))

(event Input|EnhancedActionEvents|EnhancedInputActionIA_Movimiento
  (params (ActionValue :type Float%20%28double-precision%29) (ElapsedSeconds :type Float%20%28double-precision%29) (TriggeredSeconds :type Float%20%28double-precision%29) (InputAction :type Input%20Action%20Object%20Reference :default "/Game/Character/Input/Action/IA_Movimiento.IA_Movimiento"))
  ;[1 1 1] MOVIMIENTO
  (:Triggered
    (Pawn|Input|AddMovementInput "1.200000,0.000000,0.000000" ActionValue false)
    (if (not (Character|IsJumpProvidingForce))
      (if (not (AI|Components|NavMovement|IsFalling (Variables|Character|GetCharacterMovement)))
        (Sprite|SetFlipbook (Variables|Default|GetSprite) "/Game/Assets/CHILLBOY_BASIC_ANIMATION/RUN/SPR_CHILL_BOY_Running.SPR_CHILL_BOY_Running"))))
  (:Completed
    (if (not (AI|Components|NavMovement|IsFalling (Variables|Character|GetCharacterMovement)))
      (Sprite|SetFlipbook (Variables|Default|GetSprite) "/Game/Assets/CHILLBOY_BASIC_ANIMATION/IDLE/SPR_CHILL_BOY_Chill_Idle.SPR_CHILL_BOY_Chill_Idle")
      (if true
        (Transformation|SetRelativeScale3D (Variables|Default|GetSprite) "-1.000000,1.000000,1.000000")
        (else
          (Transformation|SetRelativeScale3D (Variables|Default|GetSprite) "1.000000,1.000000,1.000000"))))))

(event EventBeginPlay
  ;[1 1 1] BEGINPLAY
  (bind _asplayer_controller (Utilities|Casting|CastToPlayerController (Pawn|GetController)))
  (Input|AddMappingContext (PlayerController|LocalPlayerSubsystems|GetEnhancedInputLocalPlayerSubsystem _asplayer_controller) "/Game/Character/Input/IMC_CharacterMapping.IMC_CharacterMapping" 0 "(bIgnoreAllPressedKeysUntilRelease=True,bForceImmediately=False,bNotifyUserSettings=False)"))

(event EventOnLanded
  (params (Hit :type Hit%20Result%20Structure%20%28by%20ref%29))
  ;[1 1 1] LANDED
  (Sprite|SetFlipbook (Variables|Default|GetSprite) "/Game/Assets/CHILLBOY_BASIC_ANIMATION/IDLE/SPR_CHILL_BOY_Chill_Idle.SPR_CHILL_BOY_Chill_Idle"))

(event EventTick
  (params (DeltaSeconds :type Float%20%28single-precision%29))
  ;[1 1 1] EVENT TICK _ ACTUALIZAR ANIMACION
  (if (>= (.x (Transformation|GetVelocity)) 0.0)
    (if (> (.x (Transformation|GetVelocity)) 0.0)
      (bind _output_get (Variables|Default|SetLastScale "-1.000000,1.000000,1.000000"))
      (Transformation|SetRelativeScale3D (Variables|Default|GetSprite) _output_get)
      (else
        (Transformation|SetRelativeScale3D (Variables|Default|GetSprite) (Variables|Default|GetLastScale))))
    (else
      (bind _output_get_2 (Variables|Default|SetLastScale "1.000000,1.000000,1.000000"))
      (Transformation|SetRelativeScale3D (Variables|Default|GetSprite) _output_get_2))))

(fn ConstructionScript)