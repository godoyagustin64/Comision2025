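; BP_Caja is a box Blueprint that prints its stats and rotates continuously, apparently as a test or debug object.
; BeginPlay starts an endless short-Delay loop that prints name, health, damage, speed, rotation speed and armor, then adds a small fixed local rotation.
; The rotation speed variable is only printed and does not drive the rotation.
; Tick separately prints the GetFramePace value under a fixed key.
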(event EventBeginPlay
  (Development|PrintString (Utilities|String|Append "Nombre:  
" (Variables|Default|GetNombre) " 
Vida actual: 
" (Utilities|String|ToString(Float) (Variables|Default|GetVida)) " 
Vida Máxima: 
" (Utilities|String|ToString(Float) (Variables|Default|GetVida%20Maxima)) " 
Daño: 
" (Utilities|String|ToString(Float) (Variables|Default|GetDaño)) " 
Velocidad: 
" (Utilities|String|ToString(Vector) (Variables|Default|GetVelocidad)) " 
Velocidad rotacion: 
" (Utilities|String|ToString(Rotator) (Variables|Default|GetVelocidadDeRotacion)) " 
Armadura: 
" (Utilities|String|ToString(Float) (Variables|Default|GetArmadura))) true true "(R=0.000000,G=0.660000,B=1.000000,A=1.000000)" 1e+01 :!label _label)
  (Utilities|FlowControl|Delay 0.01)
  (Transformation|AddActorLocalRotation "0.000000,0.000000,0.100000" false false)
  (goto _label))

(event EventTick
  (params (DeltaSeconds :type Float%20%28single-precision%29))
  (Development|PrintString (Utilities|String|ToString(Integer) (Class|GameUserSettings|GetFramePace)) true true "(R=0.000000,G=0.660000,B=1.000000,A=1.000000)" 2.0 "1"))

(fn ConstructionScript)